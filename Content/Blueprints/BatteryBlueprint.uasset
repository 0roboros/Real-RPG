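; Battery pickup Blueprint that shows a sparking discharge beam to the player character when picked up.
; On BeginPlay, Init sets the discharge time to the length of MyCharacter's PowerUpTimeline.
; OnPickedUp attaches a beam emitter to the pickup mesh and re-targets it to the player's spine socket through a short delay loop.
; The parent pickup logic is deferred until the discharge time elapses.
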(event EventOnPickedUp
  (bind _returnvalue (Effects|SpawnEmitterAttached "/Game/StarterContent/Particles/P_Sparks.P_Sparks" (Variables|Default|GetPickupMesh) "None" "0, 0, 0" "0, 0, 0" "SnapToTarget"))
  (Class|ParticleSystemComponent|SetBeamTargetPoint _returnvalue 0 (Transformation|GetSocketLocation (Variables|/Script/Engine.Character|GetMesh (Game|GetPlayerCharacter 0)) "spine_03") :!label _label)
  (Utilities|FlowControl|Sequence
    (:then_0
      (Utilities|FlowControl|Delay (Variables|Default|GetDischarge%20Time))
      (|CallParentFunction))
    (:then_1
      (Utilities|FlowControl|Delay 0.1)
      (goto _label))))

(event EventBeginPlay
  (CallFunction|Init))

(fn ConstructionScript)

(fn Init
  (bind _asmycharacter_c (Utilities|Casting|CastToMyCharacter (Game|GetPlayerCharacter 0)))
  (Variables|Default|SetDischarge%20Time (Components|Timeline|GetTimelineLength (Variables|/Game/Blueprints/MyCharacter.MyCharacter_C|GetPowerUpTimeline _asmycharacter_c))))